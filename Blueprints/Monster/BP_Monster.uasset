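; Monster actor for a side-on 2D game that takes hits from BP_Hero and pays out gold and experience when killed.
; Each tick it pins its Y position and updates its health bar widget.
; Damage plays a hit animation; at zero health it flags dead briefly, then refills health in place rather than being destroyed.
; The monster also drives hero level-ups, carrying over surplus experience and raising the next threshold geometrically.
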(event `self.ReceiveTick`
  (params (DeltaSeconds :type "Float (single-precision)"))
  (`self.LockY`)
  (bind _asmonster_hud (cast `/Game/Blueprints/Monster/Monster_HUD` (`WidgetComponent.GetWidget` (`self.health_Bar`))))
  (`ProgressBar.SetPercent` (`/Game/Blueprints/Monster/Monster_HUD.health_progress_bar` _asmonster_hud) (/ (`self.health`) (`self.max_health`))))

(event `LockY`
  (bind (_returnvalue_x _returnvalue_y _returnvalue_z) (`KismetMathLibrary.BreakVector` (`self.K2_GetActorLocation`)))
  (`self.K2_SetActorLocation` (`KismetMathLibrary.MakeVector` _returnvalue_x 0.0 _returnvalue_z)))

(event `self.ReceiveAnyDamage`
  (params (Damage :type "Float (single-precision)") (DamageType :type "DamageType Object Reference") (InstigatedBy :type "Controller Object Reference") (DamageCauser :type "Actor Object Reference"))
  (bind _bp_hero (`self.BP_Hero`))
  (bind _bp_hero_2 (`self.BP_Hero`))
  (bind _bp_hero_3 (`self.BP_Hero`))
  (bind _bp_hero_4 (`self.BP_Hero`))
  (bind _total_exp (`/Game/Blueprints/Hero/BP_Hero.total_exp` _bp_hero_2))
  (bind _returnvalue (+ (`/Game/Blueprints/Hero/BP_Hero.curr_exp` _bp_hero_3) (`self.give_exp`)))
  (`PaperZDAnimInstance.JumpToNode` (`PaperZDAnimationComponent.AnimInstance` (`self.AnimationComponent`)) "damaged" "None")
  (bind _output_get (set `self.Hero` DamageCauser))
  (bind _asbp_hero (cast `/Game/Blueprints/Hero/BP_Hero` _output_get))
  (set `self.BP_Hero` _asbp_hero)
  (bind _output_get_2 (set `self.health` (- (`self.health`) Damage)))
  (if (<= _output_get_2 0.0)
    (set `/Game/Blueprints/Hero/BP_Hero.gold` (+ (`/Game/Blueprints/Hero/BP_Hero.goldPerKill` _bp_hero_4) (`/Game/Blueprints/Hero/BP_Hero.gold` _bp_hero_4)) (`self.BP_Hero`))
    (set `self.isDead` true)
    (`KismetSystemLibrary.Delay` 0.2)
    (set `self.isDead` false)
    (set `self.health` (`self.max_health`))
    (if (>= _returnvalue (`/Game/Blueprints/Hero/BP_Hero.total_exp` _bp_hero_3))
      (set `/Game/Blueprints/Hero/BP_Hero.Level` (+ (`/Game/Blueprints/Hero/BP_Hero.Level` _bp_hero) 1) _bp_hero)
      (set `/Game/Blueprints/Hero/BP_Hero.curr_exp` (- (+ (`/Game/Blueprints/Hero/BP_Hero.curr_exp` (`self.BP_Hero`)) (`self.give_exp`)) _total_exp) _bp_hero_2)
      (set `/Game/Blueprints/Hero/BP_Hero.total_exp` (* _total_exp 1.1) _bp_hero_2)
      (`/Game/Blueprints/Hero/BP_Hero.OnLevelUp` (`self.BP_Hero`))
      (else
        (set `/Game/Blueprints/Hero/BP_Hero.curr_exp` _returnvalue (`self.BP_Hero`))))
    (else
      (`KismetSystemLibrary.PrintString` (`KismetStringLibrary.Conv_DoubleToString` (`self.health`))))))

(fn `UserConstructionScript`)